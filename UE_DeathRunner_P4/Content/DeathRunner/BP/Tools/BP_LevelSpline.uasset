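; BP_LevelSpline is a level-building tool that generates a floor and side walls along an editable spline.
; The construction script runs MeshSplinePath for the floor, a left wall, and two right-wall layers, one of them in glass.
; MeshSplinePath splits the spline by mesh length and adds a spline mesh component per segment, offsetting and scaling it, with tangents clamped to segment length for clean bends.
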(event EventBeginPlay)

(event Collision|EventActorBeginOverlap
  (params (OtherActor :type Actor%20Object%20Reference)))

(event EventTick
  (params (DeltaSeconds :type Float%20%28single-precision%29)))

(fn ConstructionScript
  (bind _wallscale (Variables|Wall|GetWallScale))
  (bind _wallscale_2 (Variables|Wall|GetWallScale))
  (bind _walloffset (Variables|Wall|GetWallOffset))
  (bind _globaloffset (Variables|Wall|GetGlobalOffset))
  (CallFunction|MeshSplinePath (Variables|Floor|GetFloorMesh) (Variables|Floor|GetFloorMeshLength) (Variables|Floor|GetFloorSpline) "1.000000,1.000000,1.000000" "0, 0, 0" (Variables|Default|GetGlobalMat))
  ;[1 1 1] Left
  (CallFunction|MeshSplinePath (Variables|Wall|GetWallMesh) (Variables|Wall|GetWallMeshLength) (Variables|Floor|GetFloorSpline) (Variables|Wall|GetWallScale) (+ (Math|Vector|MakeVector (.x _walloffset) (* (.y _walloffset) -1.0) (.z _walloffset)) _globaloffset) (Variables|Default|GetGlobalMat))
  ;[1 1 1] Right
  (CallFunction|MeshSplinePath (Variables|Wall|GetWallMesh) (Variables|Wall|GetWallMeshLength) (Variables|Floor|GetFloorSpline) (Math|Vector|MakeVector (.x _wallscale) (* (.y _wallscale) 2.0) 1.0) (+ (Math|Vector|MakeVector (.x _walloffset) (.y _walloffset) 5e+01) _globaloffset) (Variables|Default|GetGlobalMat))
  (CallFunction|MeshSplinePath (Variables|Wall|GetWallMesh) (Variables|Wall|GetWallMeshLength) (Variables|Floor|GetFloorSpline) (Math|Vector|MakeVector (.x _wallscale_2) (* (.y _wallscale_2) 2.0) (.z _wallscale_2)) (+ (Math|Vector|MakeVector (.x _walloffset) (.y _walloffset) (.z _walloffset)) _globaloffset) "/Game/Art/Material/MI_Glass.MI_Glass"))

(fn MeshSplinePath
  (params (Mesh :type Static%20Mesh%20Object%20Reference) (MeshLength :type Float%20%28double-precision%29) (Spline :type Spline%20Component%20Object%20Reference) (WallScale :type Vector) (WallOffset :type Vector) (Mat :type Material%20Instance%20Object%20Reference))
  (bind _returnvalue (Spline|GetSplineLength Spline))
  (bind _returnvalue_2 (/ _returnvalue MeshLength))
  (bind _returnvalue_3 (Math|Float|Truncate _returnvalue_2))
  (if (> _returnvalue_3 0)
    (for _index (range 0 _returnvalue_3)
      (bind _returnvalue_4 (AddComponent|AddSplineMeshComponent false))
      (Rendering|Material|SetMaterial _returnvalue_4 0 Mat)
      (Components|StaticMesh|SetStaticMesh _returnvalue_4 Mesh)
      (Transformation|SetRelativeScale3D _returnvalue_4 WallScale)
      (Transformation|SetRelativeLocation _returnvalue_4 WallOffset false false)
      (SplineMesh|SetStartandEnd _returnvalue_4 (Spline|GetLocationatDistanceAlongSpline Spline (* _index MeshLength) "Local") (Math|Vector|ClampVectorSize (Spline|GetTangentatDistanceAlongSpline Spline (* _index MeshLength) "Local") 1.0 MeshLength) (Spline|GetLocationatDistanceAlongSpline Spline (* (+ _index 1) MeshLength) "Local") (Math|Vector|ClampVectorSize (Spline|GetTangentatDistanceAlongSpline Spline (* (+ _index 1) MeshLength) "Local") 1.0 MeshLength) true :!class /Script/Engine.SplineMeshComponent)
      (Transformation|AttachComponentToComponent _returnvalue_4 Spline "None" "KeepRelative" "KeepRelative" "KeepRelative" true))))