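; BP_DeathCollider is a trap collision volume that currently only prints debug messages on contact, with no kill or damage logic.
; Box overlaps report whether the other actor is the player character.
; Box hits print a similar message but compare HitComponent, not the other actor, against the player.
; The construction script sizes the box by multiplying its current scaled extent by the BoxExtend variable.
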(event OnComponentBeginOverlap(Box)
  (params (OverlappedComponent :type Primitive%20Component%20Object%20Reference) (OtherActor :type Actor%20Object%20Reference) (OtherComp :type Primitive%20Component%20Object%20Reference) (OtherBodyIndex :type Integer) (bFromSweep :type Boolean) (SweepResult :type Hit%20Result%20Structure%20%28by%20ref%29))
  (if (== OtherActor (Game|GetPlayerCharacter 0))
    (Development|PrintString "Overlap with Player")
    (else
      (Development|PrintString "Overlap with Something"))))

(event OnComponentHit(Box)
  (params (HitComponent :type Primitive%20Component%20Object%20Reference) (OtherActor :type Actor%20Object%20Reference) (OtherComp :type Primitive%20Component%20Object%20Reference) (NormalImpulse :type Vector :default "0, 0, 0") (Hit :type Hit%20Result%20Structure%20%28by%20ref%29))
  (if (== HitComponent (Game|GetPlayerCharacter 0))
    (Development|PrintString "Hit with Player")
    (else
      (Development|PrintString "Hit with Something"))))

(fn ConstructionScript
  (bind _box (Variables|Default|GetBox))
  (Components|Box|SetBoxExtent _box (* (Variables|Default|GetBoxExtend) (Components|Box|GetScaledBoxExtent _box)) true))