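; BP_MovingPlatform_L is a moving platform trap that slides from its starting location by the EndPos offset.
; Tick plays a Timeline whose Movement track lerps the actor's location from the position stored at BeginPlay.
; A Box overlap toggles player 0 input on the actor, though no input events use it.
; The nodes deriving EndPos from the up vector and Offset are disconnected, so EndPos keeps its default.
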(event OnComponentBeginOverlap(Box)
  (params (OverlappedComponent :type Primitive%20Component%20Object%20Reference) (OtherActor :type Actor%20Object%20Reference) (OtherComp :type Primitive%20Component%20Object%20Reference) (OtherBodyIndex :type Integer) (bFromSweep :type Boolean) (SweepResult :type Hit%20Result%20Structure%20%28by%20ref%29))
  (Input|EnableInput (Game|GetPlayerController 0)))

(event OnComponentEndOverlap(Box)
  (params (OverlappedComponent :type Primitive%20Component%20Object%20Reference) (OtherActor :type Actor%20Object%20Reference) (OtherComp :type Primitive%20Component%20Object%20Reference) (OtherBodyIndex :type Integer))
  (Input|DisableInput (Game|GetPlayerController 0)))

(event EventTick
  (params (DeltaSeconds :type Float%20%28single-precision%29))
  (bind _movement (Timeline|Timeline Play)
    (:Update
      (Transformation|SetActorLocationAndRotation (Math|Vector|Lerp(Vector) (Variables|Default|GetStartPos) (+ (Variables|Default|GetStartPos) (Variables|Default|GetEndPos)) _movement) "0, 0, 0"))))

(event EventBeginPlay
  ;[1 1 1] Initialisation
  (Variables|Default|SetStartPos (Transformation|GetActorLocation)))

(fn ConstructionScript)