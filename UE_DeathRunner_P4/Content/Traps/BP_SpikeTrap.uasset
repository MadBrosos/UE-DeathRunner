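; Spike trap actor that raises a spike mesh to an Arrow component's position, then resets it.
; ActivateSpike waits, moves the mesh to the arrow's relative location, waits again, then calls DeactivateSpike to snap it back to the origin saved on BeginPlay.
; The box overlap only prints a debug message; nothing in this Blueprint calls ActivateSpike.
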(event OnComponentBeginOverlap(Box)
  (params (OverlappedComponent :type Primitive%20Component%20Object%20Reference) (OtherActor :type Actor%20Object%20Reference) (OtherComp :type Primitive%20Component%20Object%20Reference) (OtherBodyIndex :type Integer) (bFromSweep :type Boolean) (SweepResult :type Hit%20Result%20Structure%20%28by%20ref%29))
  (Development|PrintString "Overlap with something"))

(event Custom|Activate%20Spike
  (Utilities|FlowControl|Delay (Variables|Default|GetTimeBeforeAppear))
  (Components|MoveComponentTo (Variables|Default|GetSpikeMesh) (Variables|/Script/Engine.SceneComponent|GetRelativeLocation (Variables|Default|GetArrow)) "0, 0, 0" false false 0.2 false)
  (Utilities|FlowControl|Delay (Variables|Default|GetTimeBeforeReset))
  (CallFunction|DeactivateSpike))

(event Custom|Deactivate%20Spike
  (Transformation|SetRelativeLocation (Variables|Default|GetSpikeMesh) (Variables|Default|GetOriginPos) false false))

(event Collision|EventActorBeginOverlap
  (params (OtherActor :type Actor%20Object%20Reference)))

(event EventTick
  (params (DeltaSeconds :type Float%20%28single-precision%29)))

(event EventBeginPlay
  (bind _output_get (Variables|Default|SetOriginPos (Variables|/Script/Engine.SceneComponent|GetRelativeLocation (Variables|Default|GetSpikeMesh))))
  (Transformation|SetRelativeLocation (Variables|Default|GetSpikeMesh) _output_get false false))

(fn ConstructionScript)