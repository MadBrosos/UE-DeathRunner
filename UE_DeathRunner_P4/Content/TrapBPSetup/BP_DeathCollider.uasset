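; BP_DeathCollider is a trap collider that kills the first-person player on contact.
; Capsule overlap casts the other actor to BP_FirstPersonCharacter and calls Die on success, printing a debug message either way.
; The capsule's hit event only prints, and its branch is fixed to true, so it always reports the player.
; The construction script does nothing, as its Box extent scaling by BoxExtend is disconnected.
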(event OnComponentBeginOverlap(Capsule)
  (params (OverlappedComponent :type Primitive%20Component%20Object%20Reference) (OtherActor :type Actor%20Object%20Reference) (OtherComp :type Primitive%20Component%20Object%20Reference) (OtherBodyIndex :type Integer) (bFromSweep :type Boolean) (SweepResult :type Hit%20Result%20Structure%20%28by%20ref%29))
  (bind _asbp_first_person_character (Utilities|Casting|CastToBP_FirstPersonCharacter OtherActor)
    (:then
      (Default|Die _asbp_first_person_character)
      (Development|PrintString "Overlap with Player"))
    (:CastFailed
      (Development|PrintString "Overlap with Something"))))

(event OnComponentHit(Capsule)
  (params (HitComponent :type Primitive%20Component%20Object%20Reference) (OtherActor :type Actor%20Object%20Reference) (OtherComp :type Primitive%20Component%20Object%20Reference) (NormalImpulse :type Vector :default "0, 0, 0") (Hit :type Hit%20Result%20Structure%20%28by%20ref%29))
  (if true
    (Development|PrintString "Hit with Player")
    (else
      (Development|PrintString "Hit with Something"))))

(fn ConstructionScript)