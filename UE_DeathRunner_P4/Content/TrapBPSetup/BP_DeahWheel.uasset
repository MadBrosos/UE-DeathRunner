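; BP_DeahWheel is a rotating wheel actor, apparently a trap, that spins around its local roll axis.
; An Interact event toggles a LaunchRotation flag on and off.
; While the flag is set, Tick adds local roll rotation scaled by SpeedRotation and delta time, keeping the spin frame-rate independent.
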(event EventInteract
  ;[1 1 1] Enable Rotator
  (if (Variables|Default|GetLaunchRotation)
    (Variables|Default|SetLaunchRotation false)
    (else
      (Variables|Default|SetLaunchRotation true))))

(event EventTick
  (params (DeltaSeconds :type Float%20%28single-precision%29))
  ;[1 1 1] Rotator
  (if (Variables|Default|GetLaunchRotation)
    (Transformation|AddActorLocalRotation (Math|Rotator|MakeRotator (* DeltaSeconds (Variables|Default|GetSpeedRotation)) 0.0 0.0) false false)))

(fn ConstructionScript)