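; BP_InteractPlatform is a platform the player toggles with Interact to either move or rescale it.
; Overlapping its box enables player input, and leaving disables it; Interact flips a boolean.
; Tick plays or reverses a timeline from that boolean, lerping location toward start plus EndPos, or scale toward a target, depending on Type.
; Disconnected leftover nodes include an up-vector offset calculation for EndPos.
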(event OnComponentBeginOverlap(Box)
  (params (OverlappedComponent :type Primitive%20Component%20Object%20Reference) (OtherActor :type Actor%20Object%20Reference) (OtherComp :type Primitive%20Component%20Object%20Reference) (OtherBodyIndex :type Integer) (bFromSweep :type Boolean) (SweepResult :type Hit%20Result%20Structure%20%28by%20ref%29))
  (Input|EnableInput (Game|GetPlayerController 0)))

(event OnComponentEndOverlap(Box)
  (params (OverlappedComponent :type Primitive%20Component%20Object%20Reference) (OtherActor :type Actor%20Object%20Reference) (OtherComp :type Primitive%20Component%20Object%20Reference) (OtherBodyIndex :type Integer))
  (Input|DisableInput (Game|GetPlayerController 0)))

(event EventInteract
  ;[1 1 1] Interact
  (if (Variables|Default|GetInteract?)
    (Variables|Default|SetInteract? false)
    (else
      (Variables|Default|SetInteract? true))))

(event EventTick
  (params (DeltaSeconds :type Float%20%28single-precision%29))
  (if (Variables|Default|GetInteract?)
    (bind _movement (Timeline|Timeline Play)
      (:Update
        (switch Utilities|FlowControl|Switch|SwitchonE_PlatformType (Variables|Default|GetType)
          (:NewEnumerator0
            ;[1 1 1] Movement
            (Transformation|SetActorLocationAndRotation (Math|Vector|Lerp(Vector) (Variables|Default|GetStartPos) (+ (Variables|Default|GetStartPos) (Variables|Movement|GetEndPos)) _movement) "0, 0, 0"))
          (:NewEnumerator1
            (Transformation|SetActorScale3D (Math|Vector|Lerp(Vector) (Variables|Scale|GetOriginalScale) (Math|Conversions|ToVector(Float) (Variables|Scale|GetScale)) _movement))))))
    (else
      (Timeline|Timeline Reverse))))

(event EventBeginPlay
  ;[1 1 1] Initialisation
  (Variables|Default|SetStartPos (Transformation|GetActorLocation))
  (Variables|Scale|SetOriginalScale (Transformation|GetActorScale3D)))

(fn ConstructionScript)